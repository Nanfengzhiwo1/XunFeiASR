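; BP_ASR is a push-to-talk speech recognition test actor that prints recognized speech to the screen.
; On BeginPlay it spawns a SpeechActor, initializes it and enables input for the first player.
; Holding Space opens recording; releasing it stops, waits briefly, then fetches and prints the result.
; EndPlay shuts the speech engine down and clears the reference.
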(event Custom|Result
  (Utilities|FlowControl|Delay 0.2)
  (bind _returnvalue (Class|SpeechActor|SpeechResult (Variables|Default|GetSpeech)))
  (Development|PrintString _returnvalue true true "(R=0.000000,G=0.660000,B=1.000000,A=1.000000)" 2e+01))

(event EventBeginPlay
  (bind _returnvalue (Game|SpawnActorfromClass "/Script/XunFei.SpeechActor" (Math|Transform|MakeTransform "0, 0, 0") "Undefined" 0 0))
  (Variables|Default|SetSpeech _returnvalue)
  (Utilities|IsValid (Variables|Default|GetSpeech)
    (:Is%20Valid
      (Class|SpeechActor|SpeechInit (Variables|Default|GetSpeech))
      (Input|EnableInput (Game|GetPlayerController 0)))))

(event EventEndPlay
  (params (EndPlayReason :type EEndPlayReason%20Enum :default "Destroyed"))
  (Utilities|IsValid (Variables|Default|GetSpeech)
    (:Is%20Valid
      (Class|SpeechActor|SpeechQuit (Variables|Default|GetSpeech))
      (Variables|Default|SetSpeech 0))))

(event Input|KeyboardEvents|SpaceBar
  (params (Key :type Key%20Structure :default "None"))
  (bind _speech (Variables|Default|GetSpeech))
  (:Pressed
    (Utilities|IsValid _speech
      (:Is%20Valid
        (Class|SpeechActor|SpeechOpen (Variables|Default|GetSpeech))
        (Development|PrintString "SpeechOpen"))))
  (:Released
    (Utilities|IsValid _speech
      (:Is%20Valid
        (Class|SpeechActor|SpeechStop (Variables|Default|GetSpeech))
        (CallFunction|Result)))))

(fn ConstructionScript)